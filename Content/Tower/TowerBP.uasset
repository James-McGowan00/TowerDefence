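; Tower defense turret that targets AiRunners in range and fires projectiles at them on a reload delay.
; A struct sets mesh, range and attack stats, and upgrades replace it from a data table row.
; Sphere overlaps set and clear the target, while Tick shoots or runs sphere traces that store a candidate only in TempTarget.
; Added XP raises the level against thresholds, scaling projectile damage.
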(event OnComponentBeginOverlap(Sphere)
  (params (OverlappedComponent :type Primitive%20Component%20Object%20Reference) (OtherActor :type Actor%20Object%20Reference) (OtherComp :type Primitive%20Component%20Object%20Reference) (OtherBodyIndex :type Integer) (bFromSweep :type Boolean) (SweepResult :type Hit%20Result%20Structure%20%28by%20ref%29))
  ;[1 1 1] Once a target enters the sphere collision, it will be targeted
  (Utilities|IsValid (Variables|Default|GetTowerTarget)
    (:Is%20Not%20Valid
      (bind _asai_runner (Utilities|Casting|CastToAiRunner OtherActor))
      (Variables|Default|SetTowerTarget _asai_runner))))

(event OnComponentEndOverlap(Sphere)
  (params (OverlappedComponent :type Primitive%20Component%20Object%20Reference) (OtherActor :type Actor%20Object%20Reference) (OtherComp :type Primitive%20Component%20Object%20Reference) (OtherBodyIndex :type Integer))
  ;[1 1 1] Once it leaves the target it will reset what it is targeting at
  (if (== (Variables|Default|GetTowerTarget) OtherActor)
    (Variables|Default|SetTowerTarget 0)))

(event Custom|Tower
  (bind _tower_struct (Variables|Default|GetTower%20Struct))
  (bind (_name _damage _range _firerate _cost _canupgrade _upgradetotower _attacktype _splash _splashradius _splashdamage _mesh) (Utilities|Struct|BreakTower _tower_struct))
  ;[1 1 1] Sets the static mesh of the tower and its range
  (Components|StaticMesh|SetStaticMesh (Variables|Default|GetStaticMesh) _mesh)
  (Components|Sphere|SetSphereRadius (Variables|Default|GetSphere) _range true))

(event Custom|Shoot
  (bind _tower_struct (Variables|Default|GetTower%20Struct))
  (bind (_name _damage _range _firerate _cost _canupgrade _upgradetotower _attacktype _splash _splashradius _splashdamage) (Utilities|Struct|BreakTower _tower_struct))
  ;[1 1 1] This will get a target, spawn a projectile with its fire rate and the projectile will follow the target
  (Variables|Default|SetReload true)
  (switch Utilities|FlowControl|Switch|SwitchonAttackTypes _attacktype
    (:NewEnumerator0
      _)
    (:NewEnumerator1
      _))
  (Game|SpawnActorfromClass "/Game/Tower/TowerProjectile.TowerProjectile_C" (Transformation|GetActorTransform) "Undefined" 0 (Variables|Default|GetTowerTarget) (* (+ (/ (Math|Conversions|ToFloat(Integer) (Variables|Default|GetCurrentLevel)) 1e+01) 1.0) _damage) self _attacktype _splash _splashradius _splashdamage 0)
  (Utilities|FlowControl|Delay _firerate)
  (Variables|Default|SetReload false))

(event Custom|CheckForNewTarget
  (bind _returnvalue (Transformation|GetActorLocation))
  ;[1 1 1] This is the code that looks for the targets within the collision. It does this by using line traces, which track the AI runner
  (Variables|Default|SetCheckForTarget true)
  (bind (_outhits _returnvalue_2) (Collision|MultiSphereTraceForObjects _returnvalue (- _returnvalue "0,0.000000,-1.000000") (.Range (Utilities|Struct|BreakTower (Variables|Default|GetTower%20Struct))) (Utilities|Array|MakeArray "ObjectTypeQuery3") false 0 "None"))
  (if _returnvalue_2
    (bind _target (CallFunction|ClosesttoTower _outhits))
    (Utilities|IsValid _target
      (:Is%20Valid
        (Variables|Default|SetTempTarget _target))
      (:Is%20Not%20Valid
        _)))
  (Utilities|FlowControl|Delay 0.0)
  (Variables|Default|SetCheckForTarget false))

(event Custom|AddXP
  (params (XPIncrease :type Integer))
  ;[1 1 1] Allows the towers to level up
  (Variables|Default|SetExperiance (+ (Variables|Default|GetExperiance) XPIncrease))
  (CallFunction|CheckLevelUp))

(event Custom|Check%20Level%20Up
  ;[1 1 1] Allows the towers to level up
  (if (>= (Variables|Default|GetExperiance) (Utilities|Array|Get(acopy) (Variables|Default|GetUpgrade) (+ (Variables|Default|GetCurrentLevel) 1)))
    (bind _result (Math|Integer|IncrementInt (Variables|Default|GetCurrentLevel))
      (:%20%20
        (Development|PrintString (Utilities|String|Append (.Name (Utilities|Struct|BreakTower (Variables|Default|GetTower%20Struct))) ": " (Utilities|String|ToString(Integer) _result)))))))

(event Custom|Updgrade
  ;[1 1 1] Upgrade
  (if (.CanUpgrade (Utilities|Struct|BreakTower (Variables|Default|GetTower%20Struct)))
    (bind _returnvalue (Utilities|GetDataTableRow "/Game/Tower/TowerDataTable.TowerDataTable" (.UpgradeToTower (Utilities|Struct|BreakTower (Variables|Default|GetTower%20Struct))))
      (:then
        (Variables|Default|SetTower%20Struct _returnvalue)
        (CallFunction|Tower)))))

(event EventTick
  (params (DeltaSeconds :type Float%20%28single-precision%29))
  ;[1 1 1] This checks for targets, if it has a target it will shoot
  (Utilities|IsValid (Variables|Default|GetTowerTarget)
    (:Is%20Valid
      (if (not (Variables|Default|GetReload))
        (CallFunction|Shoot)))
    (:Is%20Not%20Valid
      (if (not (Variables|Default|GetCheckForTarget))
        (CallFunction|CheckforNewTarget)))))

(fn ConstructionScript)

(fn ClosesttoTower
  (params (Hit%20Results :type Array%20of%20Hit%20Result%20Structures))
  ;[1 1 1] Comment
  (for _array_element Hit%20Results
    (bind _asai_runner (Utilities|Casting|CastToAiRunner (.HitActor (Collision|BreakHitResult _array_element))))
    (Utilities|IsValid (Variables|Default|GetTowerTarget)
      (:Is%20Valid
        (if (<= (Math|Vector|VectorLength (- (Transformation|GetActorLocation) (Transformation|GetActorLocation (.HitActor (Collision|BreakHitResult _array_element))))) (Variables|Default|GetTempDistacne))
          (Variables|Default|SetTempTarget _asai_runner)
          (Variables|Default|SetTempDistacne (Math|Vector|VectorLength (- (Transformation|GetActorLocation) (Transformation|GetActorLocation (.HitActor (Collision|BreakHitResult _array_element))))))))
      (:Is%20Not%20Valid
        (Variables|Default|SetTempTarget _asai_runner)
        (Variables|Default|SetTempDistacne (Math|Vector|VectorLength (- (Transformation|GetActorLocation) (Transformation|GetActorLocation (.HitActor (Collision|BreakHitResult _array_element)))))))))
  (return (Variables|Default|GetTempTarget)))